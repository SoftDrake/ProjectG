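; Notifications helper on a game actor that posts messages to the owning player's UI notification area.
; It casts its owner to Foundation_for_Building, uses that PlayerIndex to find the Player_Controller, and calls UpdateNotifArea on its notification widget.
; The event type selects the sender name: buildings use their BuildingName, while People and Attack types still show placeholder text.
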(fn PrintMasageinNitificationArea
  (params (Notifaction%20Text :type Text) (Event%20Types :type Event_Types%20Enum :default "NewEnumerator0"))
  (bind _returnvalue (Components|GetOwner))
  (bind _asfoundation_for_building (Utilities|Casting|CastToFoundation_for_Building _returnvalue))
  (Default|UpdateNotifArea (Variables|/Game/UI/UI_Player/PlayerUI.PlayerUI_C|GetNotification_Area (Variables|/Game/Players_and_NPC/Blueprint/Players/Parent_Player/Player_Controller.Player_Controller_C|GetUI (.AsPlayer%20Controller (Utilities|Casting|CastToPlayer_Controller (Game|GetPlayerController (Variables|/Game/Business/Blueprint/Building_and_Carriage/Parent_Bilding_and_Carriage/Foundation_for_Building.Foundation_for_Building_C|GetPlayer_Index _asfoundation_for_building)))))) (Utilities|Text|ToText(String) (Utilities|Select :Index Event%20Types :NewEnumerator0 (Variables|/Game/Business/Blueprint/Building_and_Carriage/Parent_Bilding_and_Carriage/Foundation_for_Building.Foundation_for_Building_C|GetBuilding_Name _asfoundation_for_building) :NewEnumerator1 "Добавь ссылку тогда будет работать" :NewEnumerator2 "Добавь ссылку тогда будет работать")) Notifaction%20Text (Utilities|Select :Index Event%20Types :NewEnumerator0 "NewEnumerator0" :NewEnumerator1 "NewEnumerator1" :NewEnumerator2 "NewEnumerator2")))