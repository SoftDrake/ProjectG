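; Base Blueprint for people in the game, holding each person's stats, profession and workplace.
; GeneratePerson stores the given level, CoP class and place of work, then sets CraftSkills to the level for Scientist, Manager and Craftsman.
; Unconnected drafts for random first and family names and the other stats, some annotated in Russian with their intended effects, never run.
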(event EventBeginPlay)

(fn ConstructionScript)

(fn GeneratePerson
  (params (Level :type Integer) (CoP :type Category_of_Profession%20Enum :default "NewEnumerator1") (Place%20of%20Work :type Actor%20Object%20Reference))
  (bind _person_stats (Variables|Default|GetPerson_Stats))
  (Variables|/Game/Players_and_NPC/Blueprint/Parent_of_all_People/Person_Stats.Person_Stats_C|SetLevel (Variables|Default|GetPerson_Stats) Level)
  (Variables|Default|SetMy%20Place%20of%20Work Place%20of%20Work)
  (bind _output_get (Variables|Default|SetCoP CoP))
  (switch Utilities|FlowControl|Switch|SwitchonCategory_of_Profession _output_get
    (:NewEnumerator1
      _)
    (:NewEnumerator2
      _)
    (:NewEnumerator4
      _))
  (Variables|/Game/Players_and_NPC/Blueprint/Parent_of_all_People/Person_Stats.Person_Stats_C|SetCraft_Skills _person_stats (Variables|/Game/Players_and_NPC/Blueprint/Parent_of_all_People/Person_Stats.Person_Stats_C|GetLevel _person_stats)))