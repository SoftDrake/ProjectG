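; AI controller for worker NPCs that runs the movement legs of the resource gathering and delivery loop.
; It walks the worker to a resource's collection area and triggers collection on the pawn.
; For delivery, it walks to the workplace's carriage spawn area and moves inventory into the warehouse.
; If everything fits, the workplace sends the worker back to resources; otherwise leftovers stay, a warehouse-full message prints and no redispatch occurs.
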(event Custom|Go%20to%20the%20Resource
  (params (Resource_Ref :type Actor%20Object%20Reference) (Type%20Resource :type Type%20Production%20Class%20Reference))
  (AI|AIMoveTo 0 (Transformation|GetWorldLocation (Variables|/Game/Business/Blueprint/Building_and_Carriage/Resources_on_the_Map/Parent_of_Resource.Parent_of_Resource_C|GetResource%20Collection%20Area (.AsParent%20Of%20Resource (Utilities|Casting|CastToParent_of_Resource Resource_Ref)))) 0 15.0 false
    (:OnSuccess
      (Default|CollectionOfResources (.AsWorker%20Or%20Dynasty%20Member%20Parent (Utilities|Casting|CastToWorker_or_Dynasty_Member_Parent (Pawn|GetControlledPawn))) Type%20Resource))))

(event Custom|Go%20to%20the%20Warehouse%20and%20Place%20the%20Items
  (bind _returnvalue (Pawn|GetControlledPawn))
  (bind _asparent_of_all_people (Utilities|Casting|CastToParent_of_all_People _returnvalue))
  (bind _inventory_component (Variables|/Game/Players_and_NPC/Blueprint/Parent_of_all_People/Parent_of_all_People.Parent_of_all_People_C|GetInventory_Component _asparent_of_all_people))
  (bind _my_place_of_work (Variables|/Game/Players_and_NPC/Blueprint/Parent_of_all_People/Parent_of_all_People.Parent_of_all_People_C|GetMy%20Place%20of%20Work _asparent_of_all_people))
  (bind _number_pl (Variables|/Game/Players_and_NPC/Blueprint/Parent_of_all_People/Parent_of_all_People.Parent_of_all_People_C|GetNumber_PL _asparent_of_all_people))
  (bind _asfoundation_for_building (Utilities|Casting|CastToFoundation_for_Building _my_place_of_work))
  (bind _inventory (Variables|/Game/Players_and_NPC/Blueprint/Parent_of_all_People/Inventory_Component.Inventory_Component_C|GetInventory _inventory_component))
  (AI|AIMoveTo 0 (Transformation|GetWorldLocation (Variables|/Game/Business/Blueprint/Building_and_Carriage/Parent_Bilding_and_Carriage/Foundation_for_Building.Foundation_for_Building_C|GetSpawnArea_for_Carriage _asfoundation_for_building)) 0 15.0 false
    (:OnSuccess
      (for (_array_element _array_index) _inventory
        (bind (_succeess _remainder) (Default|AddinWarehouse (Variables|/Game/Business/Blueprint/Building_and_Carriage/Parent_Bilding_and_Carriage/Foundation_for_Building.Foundation_for_Building_C|GetWarehouse_Component _asfoundation_for_building) (.type_production_class _array_element) (.amount _array_element) (Pawn|GetControlledPawn)))
        (if _succeess
          (Utilities|Array|SetArrayElem _inventory _array_index (Utilities|Struct|MakeWarehouse_Struct 0 0))
          (else
            (Utilities|Array|SetArrayElem _inventory _array_index (Utilities|Struct|MakeWarehouse_Struct (.type_production_class _array_element) _remainder))
            (Development|PrintString "У рабочего еще есть предметы, а склад полон")
            (Variables|Default|SetThe%20inventory%20is%20completely%20empty%20? false))))
      (if (Variables|Default|GetThe%20inventory%20is%20completely%20empty%20?)
        (Default|SendWorkerstoResources _asfoundation_for_building (Default|CheckPLWorkerListbyPLIndex _asfoundation_for_building _number_pl) _number_pl)
        (else
          (Variables|Default|SetThe%20inventory%20is%20completely%20empty%20? true))))))

(event EventBeginPlay
  (|CallParentFunction) ; This node is disabled and will not be called.\nDrag off pins to build functionality.
)

(fn ConstructionScript
  (|CallParentFunction))