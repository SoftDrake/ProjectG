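; Parent character Blueprint for workers and dynasty members that produces resources at their place of work.
; Collection Of Resources repeats through a delayed Recursion event, accumulating points from building equipment level and the person's craft skill.
; Reaching the resource class's point cost adds items to the inventory and carries over leftover points.
; A full inventory resets points, stops the loop and has the AI controller deliver items to the warehouse.
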(event Custom|Recursion
  (params (TR :type Type%20Production%20Class%20Reference))
  (Utilities|FlowControl|Delay (Variables|CollectionofResources|GetLoop_Time))
  (CallFunction|CollectionOfResources TR))

(event EventBeginPlay
  (|CallParentFunction) ; This node is disabled and will not be called.\nDrag off pins to build functionality.
)

(event Collision|EventActorBeginOverlap
  (params (OtherActor :type Actor%20Object%20Reference)))

(fn ConstructionScript
  (|CallParentFunction))

(fn CollectionOfResources
  (params (Type_Resource :type Type%20Production%20Class%20Reference))
  (bind _typeproduction (Utilities|GetClassDefaults Type_Resource))
  (bind _success (Default|CheckInventoryIsFull? (Variables|Default|GetInventory_Component) Type_Resource (.itemswillbemade (Utilities|GetClassDefaults Type_Resource))))
  (if _success
    (Variables|CollectionofResources|SetSum_Points 0.0)
    (Default|GototheWarehouseandPlacetheItems (.AsAI%20Controller%20Of%20Worker (Utilities|Casting|CastToAI_Controller_of_Worker (Pawn|GetController self))))
    (return true)
    (else
      (bind _output_get (Variables|CollectionofResources|SetSum_Points (+ (* (* (/ (Variables|/Game/Business/Blueprint/Building_and_Carriage/Parent_Bilding_and_Carriage/Foundation_for_Building.Foundation_for_Building_C|GetEquipment_Level (.AsFoundation%20For%20Building (Utilities|Casting|CastToFoundation_for_Building (Variables|Default|GetMy%20Place%20of%20Work)))) 10) (Variables|/Game/Players_and_NPC/Blueprint/Parent_of_all_People/Person_Stats.Person_Stats_C|GetCraft_Skills (Variables|Default|GetPerson_Stats))) 1e+02) (Variables|CollectionofResources|GetSum_Points))))
      (if (>= _output_get (.points_to_create _typeproduction))
        (Variables|CollectionofResources|SetSum_Points (- _output_get (.points_to_create _typeproduction)))
        (Default|AddinInventory (Variables|Default|GetInventory_Component) Type_Resource (.itemswillbemade _typeproduction))
        (CallFunction|Recursion Type_Resource)
        (return false)
        (else
          (CallFunction|Recursion Type_Resource))))))